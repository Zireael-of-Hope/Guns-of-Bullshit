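; Main character Blueprint that handles movement speed, component setup and death.
; BeginPlay initializes the storage and health components, while Tick sets walk speed when aiming, otherwise sprint or run speed.
; Death flags the character dead, disables input for a player controller, and ragdolls player or AI characters by switching collision from capsule to physics-simulated mesh.
; A separate Stopped function halts movement immediately when flagged.
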(event `self.ReceiveBeginPlay`
  ;[0.05332 0 1] Begin Play
  (`self.- Init`))

(event `self.ReceiveTick`
  (params (DeltaSeconds :type "Float (single-precision)"))
  (if (`self.isAiming`)
    (`self.-Ironsights`)
    (else
      (`self.-Sprint`))))

(fn `- Init`
  ;[1 1 1] Storage Init
  (`/Game/Blueprints/Components/BP_Main_Component.-Init` (`self.BP_Storage_Component`))
  ;[1 1 1] Health Init
  (`/Game/Blueprints/Components/BP_Main_Component.-Init` (`self.BP_Health_Component`)))

(fn `-Death`
  (set `self.isDead` true)
  (bind _asplayer_controller (cast `PlayerController` (`self.GetInstigatorController`))
    (:`then`
      (`self.DisableInput` _asplayer_controller null))
    (:`CastFailed`
      (cast `AIController` (`self.GetInstigatorController`))))
  (`self.-EnableRagdoll`))

(fn `-EnableRagdoll`
  (`PrimitiveComponent.SetCollisionEnabled` (`self.CapsuleComponent`) "NoCollision")
  (`PrimitiveComponent.SetSimulatePhysics` (`self.Mesh`) true)
  (`PrimitiveComponent.SetCollisionEnabled` (`self.Mesh`) "PhysicsOnly")
  (`PrimitiveComponent.SetCollisionResponseToAllChannels` (`self.Mesh`) "ECR_Block"))

(fn `-Ironsights`
  (if (`self.isAiming`)
    (set `CharacterMovementComponent.MaxWalkSpeed` (`self.Walk`) (`self.CharacterMovement`))
    (else
      (set `CharacterMovementComponent.MaxWalkSpeed` (`self.Run`) (`self.CharacterMovement`)))))

(fn `-Sprint`
  (if (`self.isSprint`)
    (set `CharacterMovementComponent.MaxWalkSpeed` (`self.Sprint`) (`self.CharacterMovement`))
    (else
      (set `CharacterMovementComponent.MaxWalkSpeed` (`self.Run`) (`self.CharacterMovement`)))))

(fn `-Stopped`
  (if (`self.isStopped`)
    (`MovementComponent.StopMovementImmediately` (`self.CharacterMovement`))))

(fn `UserConstructionScript`)