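; Health component Blueprint that tracks a Health value and triggers death on its Character.
; HealthChange adds the incoming Health amount to the current value, with no upper clamp.
; When the result is zero or below, it sets Health to zero and calls Death on the Character reference.
; Init only calls the parent implementation.
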(fn `-HealthChange`
  (params (Health :type "Float (double-precision)"))
  (set `self.health` (+ Health (`self.health`)))
  (if (<= (`self.health`) 0.0)
    ;[1 1 1] Set Death
    (set `self.health` 0.0)
    (`/Game/Blueprints/BP_Main_Character_.-Death` (`self.Character`))))

(fn `-Init`
  (`parent.-Init`))