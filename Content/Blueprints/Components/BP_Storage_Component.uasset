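; Character storage component that holds carried weapons and ammo and handles equipping.
; A picked-up rifle fills a single slot on a holster socket, and WeaponChange toggles it into the current-weapon socket or drops the previous weapon ahead of the character.
; Ammo actors merge by class, and FindCurAmmo returns the stack matching the current firearm's AmmoType.
; A delayed attach event briefly sets the character's IsStopped flag.
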(event `_WeaponAttach`
  (params (Weapon :type "/Game/Blueprints/Storage/Weapon/BP_Weapon_Actor Object Reference") (SocketName :type Name))
  ;[1 1 1] Weapon  Attach
  (`|ExecutionSequence`
    (:`then_0`
      (set `/Game/Blueprints/BP_Main_Character_.isStopped` true (`self.Character`))
      (`KismetSystemLibrary.Delay` 0.7)
      (`self.- Weapon Attach` Weapon SocketName))
    (:`then_1`
      (`KismetSystemLibrary.Delay` 1.8)
      (set `/Game/Blueprints/BP_Main_Character_.isStopped` false (`self.Character`)))))

(fn `- Weapon Attach`
  (params (Weapon :type "/Game/Blueprints/Storage/Weapon/BP_Weapon_Actor Object Reference") (SocketName :type Name))
  (`Actor.K2_AttachToComponent` Weapon (`Character.Mesh` (`self.Character`)) SocketName "KeepRelative" "KeepRelative" "KeepRelative" true))

(fn `-FindCurAmmo`
  (returns (found_ammo_type :type "/Game/Blueprints/Storage/Ammo/BP_ST_ACT_Ammo Object Reference"))
  (locals (L_found_ammo_type :type "/Game/Blueprints/Storage/Ammo/BP_ST_ACT_Ammo Object Reference"))
  (bind _current_weapon (`self.current_weapon`)
    (:`then`
      (bind _asbp_weapon_fire_actor (cast `/Game/Blueprints/Storage/Weapon/Fire/BP_Weapon_Fire_Actor` _current_weapon)
        (:`then`
          (for _array_element (`self.items_ammo`)
            (if (== (`GameplayStatics.GetObjectClass` _array_element) (`/Game/Blueprints/Storage/Weapon/Fire/BP_Weapon_Fire_Actor.ammo_type` _asbp_weapon_fire_actor))
              (set `local.L_found_ammo_type` _array_element)
              (break)))
          (bind _l_found_ammo_type (`local.L_found_ammo_type`)
            (:`then`
              (return _l_found_ammo_type))
            (:`else`
              (return null))))
        (:`CastFailed`
          _)))
    (:`else`
      _))
  (return null))

(fn `-Init`
  (`parent.-Init`)
  (`KismetSystemLibrary.PrintString` "Hello"))

(fn `-ItemWeaponAdd`
  (params (NewItem :type "/Game/Blueprints/Storage/BP_Storage_Actor Object Reference (by ref)"))
  (`KismetArrayLibrary.Array_Add` (`self.items_weapon`) NewItem))

(fn `-ItemWeaponAmmo`
  (params (AmmoTypeToAdd :type "/Game/Blueprints/Storage/Ammo/BP_ST_ACT_Ammo Object Reference (by ref)"))
  (locals (L_AmmoToAdd :type "/Game/Blueprints/Storage/Ammo/BP_ST_ACT_Ammo Object Reference") (L_AmmoTypeFound :type "/Game/Blueprints/Storage/Ammo/BP_ST_ACT_Ammo Object Reference"))
  (set `local.L_AmmoToAdd` AmmoTypeToAdd)
  (for _array_element (`self.items_ammo`)
    (if (== (`GameplayStatics.GetObjectClass` _array_element) (`GameplayStatics.GetObjectClass` (`local.L_AmmoToAdd`)))
      (set `local.L_AmmoTypeFound` _array_element)
      (break)))
  (`local.L_AmmoTypeFound`
    (:`then`
      (set `/Game/Blueprints/Storage/Ammo/BP_ST_ACT_Ammo.value` (+ (`/Game/Blueprints/Storage/Ammo/BP_ST_ACT_Ammo.value` (`local.L_AmmoToAdd`)) (`/Game/Blueprints/Storage/Ammo/BP_ST_ACT_Ammo.value` (`local.L_AmmoTypeFound`))) (`local.L_AmmoTypeFound`))
      (`Actor.K2_DestroyActor` (`local.L_AmmoToAdd`)))
    (:`else`
      (`KismetArrayLibrary.Array_Add` (`self.items_ammo`) (`local.L_AmmoToAdd`))
      (`Actor.SetActorEnableCollision` (`local.L_AmmoToAdd`) false)
      (`Actor.K2_SetActorLocation` (`local.L_AmmoToAdd`) (0.0 0.0 0.0) false false)
      (`Actor.SetActorHiddenInGame` (`local.L_AmmoToAdd`) false))))

(fn `-WeaponADD`
  (params (Weapon :type "/Game/Blueprints/Storage/Weapon/BP_Weapon_Actor Object Reference"))
  (bind _asbp_weapon_fire_actor (cast `/Game/Blueprints/Storage/Weapon/Fire/BP_Weapon_Fire_Actor` Weapon))
  (bind _asbp_weapon_rifle_actor (cast `/Game/Blueprints/Storage/Weapon/Fire/Rifle/BP_Weapon_Rifle_Actor` _asbp_weapon_fire_actor))
  (`self.weapon_rifle`
    (:`then`)
    (:`else`
      (bind _output_get (set `self.weapon_rifle` _asbp_weapon_rifle_actor))
      (`Actor.SetActorEnableCollision` _output_get false)
      (`self.- Weapon Attach` _output_get "Skt_Hid_Rifle"))))

(fn `-WeaponChange`
  (params (Weapon :type "/Game/Blueprints/Storage/Weapon/BP_Weapon_Actor Object Reference"))
  (locals (L_InputWeapon :type "/Game/Blueprints/Storage/Weapon/BP_Weapon_Actor Object Reference"))
  (bind _output_get (set `local.L_InputWeapon` Weapon))
  (if (== _output_get (`self.current_weapon`))
    ;[1 1 1] Снять оружие
    (set `self.current_weapon` null)
    (`self._WeaponAttach` (`local.L_InputWeapon`) "Skt_Hid_Rifle")
    (else
      (bind _current_weapon (`self.current_weapon`)
        (:`then`
          ;[1 1 1] Снять оружие
          (`self.-WeaponDrop` _current_weapon)
          (bind _output_get_2 (set `self.current_weapon` (`local.L_InputWeapon`)))
          (`self._WeaponAttach` _output_get_2 "Skt_CurWeapon"))
        (:`else`
          (bind _output_get_3 (set `self.current_weapon` (`local.L_InputWeapon`)))
          (`self._WeaponAttach` _output_get_3 "Skt_CurWeapon"))))))

(fn `-WeaponDrop`
  (params (Weapon :type "/Game/Blueprints/Storage/Weapon/BP_Weapon_Actor Object Reference"))
  (bind _character (`self.Character`))
  (`SceneComponent.K2_DetachFromComponent` (`/Game/Blueprints/Storage/BP_Storage_Actor.DefaultSceneRoot` Weapon) "KeepRelative" "KeepRelative" "KeepRelative" true)
  (`Actor.SetActorEnableCollision` Weapon false)
  (`Actor.K2_SetActorLocation` Weapon (+ (`Actor.K2_GetActorLocation` _character) (* (`Actor.GetActorForwardVector` _character) 100.0)) false true))