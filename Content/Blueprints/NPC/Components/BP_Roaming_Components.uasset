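; NPC roaming component that moves an NPC between its assigned Places or to random reachable navmesh points.
; In place mode it cycles through the Place list, taking arrival distance and wait time from each, with random Places or an empty list falling back to random points.
; A looping timer reissues the AI move and checks distance; on arrival it runs the Place's script and schedules the next target after a delay.
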(event `self.-Init`
  (`parent.-Init`))

(event `self.-Start`
  (`parent.-Start`)
  (`self.-GoToNewTarget`)
  (set `self.Roaming` false))

(event `self.-Stop`
  (`parent.-Stop`)
  (`KismetSystemLibrary.K2_ClearAndInvalidateTimerHandle` (`self.Timer_-GoToTarget`))
  (`KismetSystemLibrary.K2_ClearAndInvalidateTimerHandle` (`self.Timer_-GoToNewTarget`))
  (set `self.PlaceLocation` (0.0 0.0 0.0))
  (set `self.Roaming` false)
  (set `self.Moving` false)
  (set `self.Waiting` false))

(fn `- Find Location`
  (returns (RandomLocation :type "Vector Structure"))
  (locals (L_LocationPlace :type "Vector Structure" :default (0.0 0.0 0.0)))
  (bind _npc (`self.NPC`))
  (bind _npc_2 (`self.NPC`))
  (bind (_randomlocation _returnvalue) (`NavigationSystemV1.K2_GetRandomReachablePointInRadius` (`Actor.K2_GetActorLocation` _npc_2) (`self.RadiusFindPoint`) (`/Game/Blueprints/NPC/BP_NPC_Character.NavMesh` _npc_2) null))
  (set `self.PlaceQuantity` (`KismetArrayLibrary.Array_Length` (`/Game/Blueprints/NPC/BP_NPC_Character.Place` (`self.NPC`))))
  (if (`self.ModePlace`)
    (if (> (`self.PlaceQuantity`) 0)
      (if (>= (`self.CurPlace`) (`self.PlaceQuantity`))
        (set `self.CurPlace` 0))
      (set `self.Place` (`|GetArrayItem` (`/Game/Blueprints/NPC/BP_NPC_Character.Place` (`self.NPC`)) (`self.CurPlace`)))
      (set `self.LengthPlace` (`/Game/Blueprints/Place/BP_Main_Place.LengthPlace` (`self.Place`)))
      (set `self.DelayGoToNewTarget` (`/Game/Blueprints/Place/BP_Main_Place.DelayPlaceWait` (`self.Place`)))
      (if (not (== (`GameplayStatics.GetObjectClass` (`self.Place`)) "/Game/Blueprints/Place/BP_Place_Random.BP_Place_Random_C"))
        (set `local.L_LocationPlace` (`Actor.K2_GetActorLocation` (`self.Place`)))
        (`/Engine/EditorBlueprintResources/StandardMacros.IncrementInt` (`self.CurPlace`)
          (:`  `
            (return (`local.L_LocationPlace`))))
        (else
          (`/Engine/EditorBlueprintResources/StandardMacros.IncrementInt` (`self.CurPlace`)
            (:`  `
              _))))))
  ;[1 1 1] Following to Random Place
  (if _returnvalue
    (return _randomlocation)
    (else
      (return (+ (`Actor.K2_GetActorLocation` _npc) (* (`Actor.GetActorForwardVector` _npc) 500.0))))))

(fn `-GoToNewTarget`
  (bind _randomlocation (`self.- Find Location`))
  (set `self.PlaceLocation` _randomlocation)
  (set `self.Moving` true)
  (set `self.Waiting` false)
  (bind _returnvalue (`KismetSystemLibrary.K2_SetTimer` null "-GoToTarget" 0.5 true))
  (set `self.Timer_-GoToTarget` _returnvalue))

(fn `-GoToTarget`
  (`AIController.MoveToLocation` (`self.NPC_AI_Controller`) (`self.PlaceLocation`) 50.0 true true false true null true)
  (if (<= (`KismetMathLibrary.VSize` (- (`Actor.K2_GetActorLocation` (`self.NPC`)) (`self.PlaceLocation`))) (`self.LengthPlace`))
    (`self.-TargetReached`)))

(fn `-TargetReached`
  (`MovementComponent.StopMovementImmediately` (`Character.CharacterMovement` (`self.NPC`)))
  (`KismetSystemLibrary.K2_ClearAndInvalidateTimerHandle` (`self.Timer_-GoToTarget`))
  (set `self.PlaceLocation` (0.0 0.0 0.0))
  (set `self.Moving` false)
  (set `self.Waiting` true)
  ;[1 1 1] Вызов скрипта у Place
  (`/Game/Blueprints/Place/BP_Main_Place.-Start` (`self.Place`) (`self.NPC`))
  (bind _returnvalue (`KismetSystemLibrary.K2_SetTimer` null "-GoToNewTarget" (`self.DelayGoToNewTarget`)))
  (set `self.Timer_-GoToNewTarget` _returnvalue))