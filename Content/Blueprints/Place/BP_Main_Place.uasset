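; BP_Main_Place is a Blueprint that tracks whether a place is active for a character and can rotate that character by a place's rotation.
; Start stores the character and sets the active flag, and Stop clears the flag while keeping the stored reference.
; While active, Rotation adds the root world rotation of the passed Place to the character's rotation as an offset, so repeated calls accumulate.
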(fn `-Rotation`
  (params (Place :type "/Game/Blueprints/Place/BP_Main_Place Object Reference"))
  (if (`self.PlaceActive`)
    (`self.K2_AddActorWorldRotation` (`self.Character`) (`SceneComponent.K2_GetComponentRotation` (`Actor.RootComponent` Place)) false false)))

(fn `-Start`
  (params (Character :type "/Game/Blueprints/BP_Main_Character_ Object Reference"))
  (set `self.Character` Character)
  (set `self.PlaceActive` true))

(fn `-Stop`
  (params (Character :type "/Game/Blueprints/BP_Main_Character_ Object Reference"))
  (set `self.PlaceActive` false))

(fn `UserConstructionScript`)