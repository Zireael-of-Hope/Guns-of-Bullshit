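; BP_Place_Tree is a tree variant of a Place Blueprint that a character can start and stop using.
; On Start it runs the parent logic, waits half a second less than DelayPlaceWait, then calls Stop on itself.
; Stop runs the parent logic and uncrouches the character.
; Tick calls Rotation on itself every frame, and the construction script only defers to the parent.
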(event `self.ReceiveTick`
  (params (DeltaSeconds :type "Float (single-precision)"))
  (`self.-Rotation` self))

(event `self.-Start`
  (params (Character :type "/Game/Blueprints/BP_Main_Character_ Object Reference"))
  (`parent.-Start` Character)
  (`KismetSystemLibrary.Delay` (- (`self.DelayPlaceWait`) 0.5))
  (`self.-Stop` Character))

(event `self.-Stop`
  (params (Character :type "/Game/Blueprints/BP_Main_Character_ Object Reference"))
  (`parent.-Stop` Character)
  (`Character.UnCrouch` Character))

(fn `UserConstructionScript`
  (`parent.UserConstructionScript`))