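; Firearm weapon actor that fires projectiles at a target and reloads from the owning character's storage.
; Shoot spends a round, spawns the configured ammo class aimed from the muzzle point with a scaled-down explosion flash, or calls Reload when empty.
; The _Reload event guards against overlapping or needless reloads and waits ReloadTime before calling Reload.
; Reload tops up the magazine from the current ammo item, leaving any surplus in storage.
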(event `_Reload`
  (bind _asbp_main_character_ (cast `/Game/Blueprints/BP_Main_Character_` (`self.GetOwner`)))
  (set `self.L_ammo` (`/Game/Blueprints/Components/BP_Storage_Component.-FindCurAmmo` (`/Game/Blueprints/BP_Main_Character_.BP_Storage_Component` _asbp_main_character_)))
  (bind _l_ammo (`self.L_ammo`)
    (:`then`
      (if (and (> (`/Game/Blueprints/Storage/Ammo/BP_ST_ACT_Ammo.value` _l_ammo) 0) (not (`self.isReloading`)) (< (`self.ammo_cur_value`) (`self.ammo_max_value`)))
        (set `self.isReloading` true)
        (`KismetSystemLibrary.Delay` (`self.reload_time`))
        (`self.-Reload`)
        (set `self.isReloading` false)))
    (:`else`)))

(fn `-Reload`
  (locals (L_ammo :type "/Game/Blueprints/Storage/Ammo/BP_ST_ACT_Ammo Object Reference") (L_ammo_value :type Integer))
  (bind _asbp_main_character_ (cast `/Game/Blueprints/BP_Main_Character_` (`self.GetOwner`)))
  (set `local.L_ammo` (`/Game/Blueprints/Components/BP_Storage_Component.-FindCurAmmo` (`/Game/Blueprints/BP_Main_Character_.BP_Storage_Component` _asbp_main_character_)))
  (bind _l_ammo (`local.L_ammo`)
    (:`then`
      (if (> (`/Game/Blueprints/Storage/Ammo/BP_ST_ACT_Ammo.value` _l_ammo) 0)
        (set `local.L_ammo_value` (+ (`self.ammo_cur_value`) (`/Game/Blueprints/Storage/Ammo/BP_ST_ACT_Ammo.value` (`local.L_ammo`))))
        (set `/Game/Blueprints/Storage/Ammo/BP_ST_ACT_Ammo.value` (`KismetMathLibrary.Max` 0 (- (`local.L_ammo_value`) (`self.ammo_max_value`))) (`local.L_ammo`))
        (set `self.ammo_cur_value` (`KismetMathLibrary.SelectInt` (`self.ammo_max_value`) (`local.L_ammo_value`) (> (`local.L_ammo_value`) (`self.ammo_max_value`))))))
    (:`else`)))

(fn `-Shoot`
  (params (Target :type "Vector Structure (by ref)"))
  (locals (L_Target :type "Vector Structure"))
  (bind _bullet_apawn_location (`self.bullet_apawn_location`))
  (bind _returnvalue (`SceneComponent.K2_GetComponentLocation` _bullet_apawn_location))
  (bind _returnvalue_2 (`KismetMathLibrary.FindLookAtRotation` _returnvalue (`local.L_Target`)))
  (set `local.L_Target` Target)
  (if (> (`self.ammo_cur_value`) 0)
    (`/Engine/EditorBlueprintResources/StandardMacros.DecrementInt` (`self.ammo_cur_value`)
      (:`  `
        (`|SpawnActorFromClass` (`self.ammo_type_spawn`) (`KismetMathLibrary.MakeTransform` _returnvalue _returnvalue_2 (`SceneComponent.K2_GetComponentScale` _bullet_apawn_location)) "AlwaysSpawn" "OverrideRootScale" self (`self.GetInstigator`))
        (`GameplayStatics.SpawnEmitterAtLocation` "/Game/Visual/StarterContent/Particles/P_Explosion.P_Explosion" _returnvalue _returnvalue_2 (0.03 0.03 0.03))))
    (else
      (`self._Reload`))))

(fn `UserConstructionScript`
  (`parent.UserConstructionScript`))